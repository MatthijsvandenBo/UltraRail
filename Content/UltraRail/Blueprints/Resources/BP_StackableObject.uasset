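; Stackable resource pickup actor that represents a pile of track, wood or iron items.
; The item type selects the base mesh, with an offset for track, in both the construction script and setup, which then adds the initial amount.
; Adding spawns copies of the mesh as components stacked upward at fixed height steps, matching the base collision profile.
; Removing pops components from the top and destroys the actor once the count reaches zero.
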(event Custom|AddToStack
  (params (AmountToAddToStack :type Integer))
  (bind _stackstaticmeshs (Variables|Default|GetStackStaticMeshs))
  (bind _staticmesh (Variables|Default|GetStaticMesh))
  (bind _returnvalue (Utilities|Array|LastIndex _stackstaticmeshs))
  (bind _output (Utilities|Array|Get(acopy) _stackstaticmeshs _returnvalue))
  (bind _returnvalue_2 (Utilities|IsValid _output))
  ;[1 1 1] Adds object to stack
  (for _index (range (Variables|Default|GetAmountOnStack) (- (+ AmountToAddToStack (Variables|Default|GetAmountOnStack)) 1))
    (bind _returnvalue_3 (AddComponent|AddStaticMeshComponent false (Math|Transform|MakeTransform (select _returnvalue_2 (+ (.location (Transformation|GetRelativeTransform (select _returnvalue_2 _output (Variables|Default|GetStaticMesh)))) "0.000000,0.000000,10.000000") (.location (Transformation|GetRelativeTransform (Variables|Default|GetStaticMesh)))) "0, 0, 0" "1.000000,1.000000,1.000000")))
    (Collision|SetCollisionProfileName _returnvalue_3 (Collision|GetCollisionProfileName _staticmesh) true :!class /Script/Engine.PrimitiveComponent)
    (Components|StaticMesh|SetStaticMesh _returnvalue_3 (Variables|/Script/Engine.StaticMeshComponent|GetStaticMesh _staticmesh))
    (Utilities|Array|Add (Variables|Default|GetStackStaticMeshs) _returnvalue_3))
  (Variables|Default|SetAmountOnStack (+ AmountToAddToStack (Variables|Default|GetAmountOnStack)))
  (Variables|Default|SetAmountToAdd 0))

(event Custom|RemoveFromStack
  (params (AmountToRemove :type Integer))
  (bind _stackstaticmeshs (Variables|Default|GetStackStaticMeshs))
  (bind _returnvalue (Utilities|Array|LastIndex _stackstaticmeshs))
  ;[1 1 1] Remove's obejct from stack and of stack is at 0 destroys stack
  (if (<= (- (Variables|Default|GetAmountOnStack) AmountToRemove) 0)
    (Actor|DestroyActor)
    (else
      (for _index (range 0 (- AmountToRemove 1))
        (Components|DestroyComponent (Utilities|Array|Get(acopy) _stackstaticmeshs _returnvalue))
        (Utilities|Array|RemoveIndex (Variables|Default|GetStackStaticMeshs) _returnvalue))
      (Variables|Default|SetAmountOnStack (- (Variables|Default|GetAmountOnStack) AmountToRemove)))))

(event Custom|SetUp
  (bind _itemtypetoset (Variables|Default|GetItemTypeToSet))
  ;[1 1 1] Beginplay
  (Variables|Default|SetItemType (Variables|Default|GetItemTypeToSet))
  (Components|StaticMesh|SetStaticMesh (Variables|Default|GetStaticMesh) (Utilities|Select :Index _itemtypetoset :NewEnumerator5 0 :NewEnumerator1 "/Game/UltraRail/Art/Assets/Rails/SM_Track.SM_Track" :NewEnumerator2 0 :NewEnumerator3 "/Game/UltraRail/Art/Assets/Resources/Wood.Wood" :NewEnumerator4 "/Game/UltraRail/Art/Assets/Resources/Iron.Iron"))
  (if (Utilities|Enum|Equal(Enum) _itemtypetoset "NewEnumerator1")
    (Transformation|SetRelativeLocation (Variables|Default|GetStaticMesh) "-50.000000,0.000000,0.000000" false false)
    (CallFunction|AddtoStack (Variables|Default|GetAmountToAdd))
    (else
      (CallFunction|AddtoStack (Variables|Default|GetAmountToAdd)))))

(event EventBeginPlay
  (bind _itemtypetoset (Variables|Default|GetItemTypeToSet))
  ;[1 1 1] Beginplay
  (Variables|Default|SetItemType (Variables|Default|GetItemTypeToSet))
  (Components|StaticMesh|SetStaticMesh (Variables|Default|GetStaticMesh) (Utilities|Select :Index _itemtypetoset :NewEnumerator5 0 :NewEnumerator1 "/Game/UltraRail/Art/Assets/Rails/SM_Track.SM_Track" :NewEnumerator2 0 :NewEnumerator3 "/Game/UltraRail/Art/Assets/Resources/Wood.Wood" :NewEnumerator4 "/Game/UltraRail/Art/Assets/Resources/Iron.Iron"))
  (if (Utilities|Enum|Equal(Enum) _itemtypetoset "NewEnumerator1")
    (Transformation|SetRelativeLocation (Variables|Default|GetStaticMesh) "-50.000000,0.000000,0.000000" false false)
    (CallFunction|AddtoStack (Variables|Default|GetAmountToAdd))
    (else
      (CallFunction|AddtoStack (Variables|Default|GetAmountToAdd)))))

(fn ConstructionScript
  (bind _itemtypetoset (Variables|Default|GetItemTypeToSet))
  (|CallParentFunction)
  (Components|StaticMesh|SetStaticMesh (Variables|Default|GetStaticMesh) (Utilities|Select :Index _itemtypetoset :NewEnumerator5 0 :NewEnumerator1 "/Game/UltraRail/Art/Assets/Rails/SM_Track.SM_Track" :NewEnumerator2 0 :NewEnumerator3 "/Game/UltraRail/Art/Assets/Resources/Wood.Wood" :NewEnumerator4 "/Game/UltraRail/Art/Assets/Resources/Iron.Iron"))
  (if (Utilities|Enum|Equal(Enum) _itemtypetoset "NewEnumerator1")
    (Transformation|SetRelativeLocation (Variables|Default|GetStaticMesh) "-50.000000,0.000000,0.000000" false false)))