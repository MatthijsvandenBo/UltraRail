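; BP_BaseResources is a base harvestable resource actor that loses HP when hit and drops a stackable item when depleted.
; ChangeHP subtracts the player's strength from HP.
; While HP remains, it sets the static mesh to one of two reduced scales, selected by HP minus one.
; At zero or below, it spawns a BP_StackableObject with its ItemType at its own transform and destroys itself.
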(event Custom|ChangeHP
  (params (PlayerStrength :type Float%20%28double-precision%29))
  ;[1 1 1] Changes the HP and size of model
  (bind _output_get (Variables|Default|SetHP (- (Variables|Default|GetHP) (* 1 PlayerStrength))))
  (if (<= _output_get 0)
    (Game|SpawnActorfromClass "/Game/UltraRail/Blueprints/Resources/BP_StackableObject.BP_StackableObject_C" (Transformation|GetActorTransform) "Undefined" "MultiplyWithRoot" 0 1 (Variables|Default|GetItemType) false 0)
    (Actor|DestroyActor)
    (else
      (Transformation|SetWorldScale3D (Variables|Default|GetStaticMesh) (Utilities|Select :Index (- (Variables|Default|GetHP) 1) :Option%200 "0.700000,0.700000,0.700000" :Option%201 "0.800000,0.800000,0.800000")))))

(fn ConstructionScript)