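; BP_CleanupBox is a temporary box volume in UltraRail's world generation that destroys unwanted actors overlapping it.
; On BeginPlay it sets its own lifespan and sizes the box from BoxSize, updating overlaps immediately.
; Each begin-overlap passes the other actor to CanBeRemoved, which allows destruction only if its class matches or derives from an entry in RemovableList.
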(event OnComponentBeginOverlap(CleanupBox)
  (params (OverlappedComponent :type Primitive%20Component%20Object%20Reference) (OtherActor :type Actor%20Object%20Reference) (OtherComp :type Primitive%20Component%20Object%20Reference) (OtherBodyIndex :type Integer) (bFromSweep :type Boolean) (SweepResult :type Hit%20Result%20Structure%20%28by%20ref%29))
  ;[1 1 1] Listen to overlaps so the actors can be removed
  (bind _canberemoved (CallFunction|CanbeRemoved OtherActor))
  (if _canberemoved
    (Actor|DestroyActor OtherActor)))

(event EventBeginPlay
  ;[1 1 1] Setup lifetime and box-extent
  (Actor|SetLifeSpan (Variables|Default|GetLifetime))
  (Components|Box|SetBoxExtent (Variables|Default|GetCleanupBox) (Variables|Default|GetBoxSize) true))

(fn ConstructionScript)

(fn CanbeRemoved
  (params (Actor :type Actor%20Object%20Reference))
  ;[1 1 1] Checks if a given actor is allowed to be removed dictated by the RemovableList array
  (for _array_element (Variables|Default|GetRemovableList)
    (if (Class|GameplayStatics|ObjectIsA Actor _array_element)
      (return true)))
  (return false))