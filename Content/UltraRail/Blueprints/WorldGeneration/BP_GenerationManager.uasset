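; Generation manager that builds the railway world at runtime, from the start area to successive end stations.
; It chains WaveFunctionCollapse chunks through collapse callbacks, alternating target-biome terrain with station-biome chunks that get an end station at randomized depth.
; After the first chunk it spawns the start station, tools, resources and locomotive in cleared areas and teleports players.
; Each train arrival triggers the next segment, then releases the brakes after a wait.
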(event Custom|OnFieldCollapsed
  (params (Success :type Boolean) (WasStartingChunk :type Boolean))
  ;[1 1 1] Listen to when start-generation is done and spawn in station and tools
  (EventDispatchers|UnbindEventfromOnFieldCollapsed (Variables|Generation|GetWaveFunctionCollapse) (delegate Custom|OnFieldCollapsed))
  (if Success
    (Utilities|FlowControl|DelayUntilNextTick)
    (CallFunction|GenerateStartFurther)
    (CallFunction|SpawnStartStation)
    (CallFunction|SpawnTools)
    (CallFunction|SpawnResources)
    (CallFunction|PutPlayers)
    (CallFunction|SetTrainStartStation)
    (else
      (Development|PrintString "Failure to generate start chunk"))))

(event Custom|SpawnStartStation
  ;[1 1 1] Clear the area and spawn the station
  (Game|SpawnActorfromClass "/Game/UltraRail/Blueprints/WorldGeneration/BP_CleanupBox.BP_CleanupBox_C" (Variables|Spawning|GetStationSpawnLocation) "AlwaysSpawn" "MultiplyWithRoot" 0 (Variables|Cleaning|GetAllowedRemovables) 1.0 "1000.000000,350.000000,15.000000" 0)
  (bind _returnvalue (Game|SpawnActorfromClass "/Game/UltraRail/Blueprints/Track/BP_StartStation.BP_StartStation_C" (Variables|Spawning|GetStationSpawnLocation) "AlwaysSpawn" "MultiplyWithRoot" 0 0))
  (Variables|StartAssets|SetStartStation _returnvalue))

(event Custom|ListenToArrival
  ;[1 1 1] Waits for the train's arrival to generate further
  (EventDispatchers|BindEventtoOnTrainArrived (Variables|Generation|GetLastGeneratedStation) (delegate Custom|OnTrainArrived)))

(event Custom|OnTrainArrived
  (params (Station :type BP%20End%20Station%20Object%20Reference) (Train :type BP%20Locomotive%20Object%20Reference))
  ;[1 1 1] Waits for the train's arrival to generate further
  (EventDispatchers|UnbindEventfromOnTrainArrived Station (delegate Custom|OnTrainArrived))
  (Utilities|FlowControl|Delay 0.5)
  (CallFunction|GenerateStartFurther)
  (Utilities|FlowControl|Delay (Variables|Generation|GetTrainStationWaitDuration))
  (Default|SetBrakingForce Train 0.0))

(event Custom|SpawnTools
  (bind _toolspawns (Variables|Spawning|GetToolSpawns))
  ;[1 1 1] Clear the area and spawn the tools in
  (bind _keys (Utilities|Map|Keys _toolspawns))
  (for _array_element _keys
    (Game|SpawnActorfromClass "/Game/UltraRail/Blueprints/WorldGeneration/BP_CleanupBox.BP_CleanupBox_C" (.Value (Utilities|Map|Find _toolspawns _array_element)) "Undefined" "MultiplyWithRoot" 0 (Variables|Cleaning|GetAllowedRemovables) 1.0 "75.000000,75.000000,50.000000" 0)
    (Game|SpawnActorfromClass _array_element (.Value (Utilities|Map|Find _toolspawns _array_element)) "AlwaysSpawn" "MultiplyWithRoot" 0 "NewEnumerator3" 0)))

(event Custom|SpawnResources
  ;[1 1 1] Spawn in starting resources
  (Game|SpawnActorfromClass "/Game/UltraRail/Blueprints/WorldGeneration/BP_CleanupBox.BP_CleanupBox_C" (Variables|Spawning|GetWoodLocation) "AlwaysSpawn" "MultiplyWithRoot" 0 (Variables|Cleaning|GetAllowedRemovables) 1.0 "75.000000,75.000000,50.000000" 0)
  (Game|SpawnActorfromClass "/Game/UltraRail/Blueprints/Resources/BP_StackableObject.BP_StackableObject_C" (Variables|Spawning|GetWoodLocation) "AlwaysSpawn" "MultiplyWithRoot" 0 6 "NewEnumerator3" false 0)
  (Game|SpawnActorfromClass "/Game/UltraRail/Blueprints/WorldGeneration/BP_CleanupBox.BP_CleanupBox_C" (Variables|Spawning|GetIronLocation) "AlwaysSpawn" "MultiplyWithRoot" 0 (Variables|Cleaning|GetAllowedRemovables) 1.0 "75.000000,75.000000,50.000000" 0)
  (Game|SpawnActorfromClass "/Game/UltraRail/Blueprints/Resources/BP_StackableObject.BP_StackableObject_C" (Variables|Spawning|GetIronLocation) "Undefined" "MultiplyWithRoot" 0 6 "NewEnumerator4" false 0))

(event Custom|GenerateStartFurther
  (bind _wavefunctioncollapse (Variables|Generation|GetWaveFunctionCollapse))
  ;[1 1 1] Generate the start further by changing the biome asset and placing the first end-station
  (Class|WaveCollapseGen|SetBiomeAsset _wavefunctioncollapse (Variables|Generation|GetTargetBiome))
  (Class|WaveCollapseGen|SetFieldWidth _wavefunctioncollapse (Variables|Generation|GetTargetGenerationWidth))
  (EventDispatchers|BindEventtoOnFieldCollapsed _wavefunctioncollapse (delegate Custom|OnNextFieldCollapsed))
  (Class|WaveCollapseGen|GenerateNextChunk _wavefunctioncollapse))

(event Custom|PutPlayers
  ;[1 1 1] Put the players at the correct position
  (bind _outactors (Actor|GetAllActorsOfClass "/Game/UltraRail/Blueprints/Core/BP_TopDownCharacter.BP_TopDownCharacter_C"))
  (for (_array_element _array_index) _outactors
    (Transformation|SetActorLocationAndRotation _array_element (.location (Utilities|Array|Get(acopy) (Variables|Spawning|GetPlayerSpawns) _array_index)) (.rotation (Utilities|Array|Get(acopy) (Variables|Spawning|GetPlayerSpawns) _array_index)) false true)))

(event Custom|SetTrainStartStation
  ;[1 1 1] Sets the correct start-station
  (Game|SpawnActorfromClass "/Game/UltraRail/Blueprints/Train/BP_Locomotive.BP_Locomotive_C" (Math|Transform|MakeTransform "0, 0, 0" "0, 0, 0" "1.000000,1.000000,1.000000") "Undefined" "MultiplyWithRoot" 0 0))

(event Custom|OnNextFieldCollapsed
  (params (Success :type Boolean) (WasStartingChunk :type Boolean))
  (bind _wavefunctioncollapse (Variables|Generation|GetWaveFunctionCollapse))
  ;[1 1 1] Generate the start further by changing the biome asset and placing the first end-station
  (EventDispatchers|UnbindEventfromOnFieldCollapsed _wavefunctioncollapse (delegate Custom|OnNextFieldCollapsed))
  (Utilities|FlowControl|DelayUntilNextTick)
  (Class|WaveCollapseGen|SetBiomeAsset _wavefunctioncollapse (Variables|Generation|GetStationBiome))
  (Class|WaveCollapseGen|SetFieldWidth _wavefunctioncollapse (Variables|Generation|GetStationGenerationWidth))
  (EventDispatchers|BindEventtoOnFieldCollapsed _wavefunctioncollapse (delegate Custom|OnFieldCollapsedEndStation))
  (Class|WaveCollapseGen|GenerateNextChunk _wavefunctioncollapse))

(event Custom|OnFieldCollapsedEndStation
  (params (Success :type Boolean) (WasStartingChunk :type Boolean))
  ;[1 1 1] Generate the start further by changing the biome asset and placing the first end-station
  (EventDispatchers|UnbindEventfromOnFieldCollapsed (Variables|Generation|GetWaveFunctionCollapse) (delegate Custom|OnFieldCollapsedEndStation))
  (CallFunction|PlaceTargetStation)
  (CallFunction|ListentoArrival))

(event Custom|PlaceTargetStation
  (bind _stationspawnlocation (Variables|Spawning|GetStationSpawnLocation))
  (bind _wavefunctioncollapse (Variables|Generation|GetWaveFunctionCollapse))
  (bind _returnvalue (Class|WaveCollapseGen|GetGenerationGridSize _wavefunctioncollapse))
  ;[1 1 1] Generates the target station and keeps a reference to it
  (bind _output_get (Variables|Spawning|SetEndStationLocation (Math|Transform|MakeTransform (Math|Vector|MakeVector (* (+ (Math|Random|RandomInteger (- (Class|WaveCollapseGen|GetGenerationFieldDepth _wavefunctioncollapse) 4)) 1) _returnvalue) (* (- (Class|WaveCollapseGen|GetGenerationOffset _wavefunctioncollapse) 5) _returnvalue) (.z (.location _stationspawnlocation))) (.rotation _stationspawnlocation) (.scale _stationspawnlocation))))
  (Game|SpawnActorfromClass "/Game/UltraRail/Blueprints/WorldGeneration/BP_CleanupBox.BP_CleanupBox_C" _output_get "Undefined" "MultiplyWithRoot" 0 (Variables|Cleaning|GetAllowedRemovables) 1.0 "300.000000,200.000000,15.000000" 0)
  (bind _returnvalue_2 (Game|SpawnActorfromClass "/Game/UltraRail/Blueprints/Track/BP_EndStation.BP_EndStation_C" (Variables|Spawning|GetEndStationLocation) "Undefined" "MultiplyWithRoot" 0 0))
  (Variables|Generation|SetLastGeneratedStation _returnvalue_2))

(event EventBeginPlay
  (bind _wavefunctioncollapse (Variables|Generation|GetWaveFunctionCollapse))
  ;[1 1 1] Listen to when start-generation is done and spawn in station and tools
  (EventDispatchers|BindEventtoOnFieldCollapsed _wavefunctioncollapse (delegate Custom|OnFieldCollapsed))
  (Class|WaveCollapseGen|SetBiomeAsset _wavefunctioncollapse (Variables|Generation|GetStationBiome))
  (Class|WaveCollapseGen|SetFieldWidth _wavefunctioncollapse (Variables|Generation|GetStationGenerationWidth))
  (Class|WaveCollapseGen|GenerateStartChunk _wavefunctioncollapse))

(fn ConstructionScript)