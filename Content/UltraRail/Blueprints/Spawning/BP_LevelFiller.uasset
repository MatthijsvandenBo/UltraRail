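; Level filler actor that populates a level with local players, one for each PlayerStart, at BeginPlay.
; Each created player with a valid Enhanced Input subsystem gets the default mapping context, and its top-down character's join-request event is bound.
; A join request currently only unbinds that character's listener and prints the controller ID.
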(event Custom|OnJoinRequested
  (params (PlyerCharacter :type BP%20Top%20Down%20Character%20Object%20Reference) (ControllerID :type Integer))
  ;[1 1 1] Listen to when a playercontroller requests to join
  (EventDispatchers|UnbindEventfromOnJoinRequested PlyerCharacter (delegate Custom|OnJoinRequested))
  (Development|PrintString (Utilities|String|ToString(Integer) ControllerID)))

(event EventBeginPlay
  ;[1 1 1] Looks for all the player starts in the level and spawn in a local player for every start
  (bind _outactors (Actor|GetAllActorsOfClass "/Script/Engine.PlayerStart"))
  (for _array_element _outactors
    (bind _returnvalue (Class|GameplayStatics|CreatePlayer -1))
    (Utilities|IsValid (PlayerController|LocalPlayerSubsystems|GetEnhancedInputLocalPlayerSubsystem _returnvalue)
      (:Is%20Valid
        (Input|AddMappingContext (PlayerController|LocalPlayerSubsystems|GetEnhancedInputLocalPlayerSubsystem _returnvalue) "/Game/UltraRail/Input/IMC_Default.IMC_Default" 0 "(bIgnoreAllPressedKeysUntilRelease=True,bForceImmediately=False,bNotifyUserSettings=False)")
        (EventDispatchers|BindEventtoOnJoinRequested (.AsBP%20Top%20Down%20Character (Utilities|Casting|CastToBP_TopDownCharacter (Pawn|GetControlledPawn _returnvalue))) (delegate Custom|OnJoinRequested))))))

(fn ConstructionScript)