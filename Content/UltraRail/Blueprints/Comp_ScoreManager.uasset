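; Score manager component that tracks how far its owning actor has travelled along the world Y axis as a distance score.
; On BeginPlay it records the owner's starting Y position, divided by 100 to convert centimetres to metres.
; Each Tick it measures the offset from that start, raising the score only when the offset exceeds the current best, and prints each new value as debug text.
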(event EventBeginPlay
  (Variables|Default|SetStartDistanceScore (/ (.y (Transformation|GetActorLocation (Components|GetOwner))) 100)))

(event EventTick
  (params (DeltaSeconds :type Float%20%28single-precision%29))
  (bind _returnvalue (Components|GetOwner))
  (bind _startdistancescore (Variables|Default|GetStartDistanceScore))
  (bind _returnvalue_2 (Transformation|GetActorLocation _returnvalue))
  (bind _returnvalue_3 (/ (.y _returnvalue_2) 100))
  (bind _returnvalue_4 (- _returnvalue_3 _startdistancescore))
  (if (not (<= _returnvalue_4 (Variables|Default|GetDistanceScore)))
    (bind _output_get (Variables|Default|SetDistanceScore _returnvalue_4))
    (Development|PrintString (Utilities|String|Append "Distance Score: " (Utilities|String|ToString(Integer) _output_get)))))