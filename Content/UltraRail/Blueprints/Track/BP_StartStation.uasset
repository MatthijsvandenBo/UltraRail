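; BP_StartStation is the starting station, holding track pieces as child actors and clearing overlapping resources from its spawn area.
; On BeginPlay it simulates placement of the last track piece by calling OnPlace on Track10 with Track9 as its argument.
; Actors that begin overlapping SpawnCollisionBox are destroyed if they match a class in the RemovableList array.
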(event OnComponentBeginOverlap(SpawnCollisionBox)
  (params (OverlappedComponent :type Primitive%20Component%20Object%20Reference) (OtherActor :type Actor%20Object%20Reference) (OtherComp :type Primitive%20Component%20Object%20Reference) (OtherBodyIndex :type Integer) (bFromSweep :type Boolean) (SweepResult :type Hit%20Result%20Structure%20%28by%20ref%29))
  ;[1 1 1] Remove overlapping resources when the starting station is placed
  (bind _canberemoved (CallFunction|CanbeRemoved OtherActor))
  (if _canberemoved
    (Actor|DestroyActor OtherActor)))

(event EventBeginPlay
  ;[1 1 1] Simulates placement on the last track-piece
  (Default|OnPlace (.AsBP%20Track (Utilities|Casting|CastToBP_Track (Variables|/Script/Engine.ChildActorComponent|GetChildActor (Variables|Default|GetTrack10)))) (.AsBP%20Track (Utilities|Casting|CastToBP_Track (Variables|/Script/Engine.ChildActorComponent|GetChildActor (Variables|Default|GetTrack9))))))

(fn ConstructionScript)

(fn CanbeRemoved
  (params (Actor :type Actor%20Object%20Reference))
  ;[1 1 1] Checks if a given actor is allowed to be removed dictated by the RemovableList array
  (for _array_element (Variables|Default|GetRemovableList)
    (if (Class|GameplayStatics|ObjectIsA Actor _array_element)
      (return true)))
  (return false))