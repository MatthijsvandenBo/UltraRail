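; BP_Track is a placeable rail track piece that extends the start station's spline as the line is built.
; On placement it spawns placement nodes at its straight, right and left points and adds a spline point.
; It compares its orientation with the previous piece using dot products, then switches that piece to a straight or corner mesh and corrects its spline point location and tangents.
; It can also remove its own spline point.
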(event Custom|OnPlace
  (params (OldTrack :type BP%20Track%20Object%20Reference))
  ;[1 1 1] Spawns all placement nodes and put them in a array
  (Variables|References|SetPreviousTrackpiece OldTrack)
  (for _array_element (Variables|PlacementNodes|GetSpawnPoints)
    (bind _returnvalue (Game|SpawnActorfromClass "/Game/UltraRail/Blueprints/BP_PlacementNode.BP_PlacementNode_C" (Math|Transform|MakeTransform (Transformation|GetWorldLocation _array_element) (Transformation|GetWorldRotation _array_element) "1.000000,1.000000,1.000000") "Undefined" "MultiplyWithRoot" self "/Game/UltraRail/Art/Assets/Rails/SM_Track.SM_Track" (CallFunction|StringtoDirection (Utilities|GetDisplayName _array_element)) 0))
    (Utilities|Array|Add (Variables|PlacementNodes|GetPlacementNodes) _returnvalue))
  (CallFunction|UpdateSplinePoint))

(event Custom|UpdatePreviousTrackpiece
  (params (Previous :type BP%20Track%20Object%20Reference))
  (bind _returnvalue (Transformation|GetActorRightVector))
  (bind _returnvalue_2 (Transformation|GetActorForwardVector Previous))
  (bind _returnvalue_3 (Math|Vector|DotProduct _returnvalue_2 _returnvalue))
  (bind _returnvalue_4 (Math|Float|NearlyEqual(Float) _returnvalue_3 1.0 0.001))
  (bind _returnvalue_5 (select _returnvalue_4 "NewEnumerator0" "NewEnumerator2"))
  ;[1 1 1] Determines the relative orientation towards the previous track by using the dot product on the forward and right vectors
  (Utilities|IsValid Previous
    (:Is%20Valid
      (if (Math|Float|NearlyEqual(Float) (Math|Vector|DotProduct (Transformation|GetActorForwardVector) _returnvalue_2) 1.0 0.001)
        (CallFunction|SetMeshDirection Previous "NewEnumerator1")
        (CallFunction|CorrectSplineAfterDirection Previous "NewEnumerator1")
        (else
          (CallFunction|SetMeshDirection Previous _returnvalue_5)
          (CallFunction|CorrectSplineAfterDirection Previous _returnvalue_5))))))

(event Custom|Remove%20SplinePoint
  ;[1 1 1] Remove's spline point
  (Spline|RemoveSplinePoint (Variables|/Game/UltraRail/Blueprints/Track/BP_StartStation.BP_StartStation_C|GetSpline (Variables|References|GetStation)) (Variables|Spline|GetSplineIndex) true))

(event Custom|UpdateSplinePoint
  (bind _station (Variables|References|GetStation))
  (bind _previoustrackpiece (Variables|References|GetPreviousTrackpiece))
  (bind _spline (Variables|/Game/UltraRail/Blueprints/Track/BP_StartStation.BP_StartStation_C|GetSpline _station))
  ;[1 1 1] Update's track and adds spline point
  (Utilities|IsValid _previoustrackpiece
    (:Is%20Valid
      (CallFunction|UpdatePreviousTrackpiece _previoustrackpiece)
      (Spline|AddSplinePoint _spline (Transformation|GetWorldLocation (Variables|Default|GetStraight)) "World" true)
      (Variables|Spline|SetSplineIndex (- (Spline|GetNumberOfSplinePoints _spline) 1)))))

(event Custom|SetMeshDirection
  (params (NewDirection :type E_Direction%20Enum :default "NewEnumerator1"))
  ;[1 1 1] Sets the mesh according to the direction
  (Components|StaticMesh|SetStaticMesh (Variables|Default|GetStaticMesh) (Utilities|Select :Index NewDirection :NewEnumerator1 "/Game/UltraRail/Art/Assets/Rails/SM_Track.SM_Track" :NewEnumerator2 "/Game/UltraRail/Art/Assets/Rails/SM_TrackCornerRight.SM_TrackCornerRight" :NewEnumerator0 "/Game/UltraRail/Art/Assets/Rails/SM_TrackCornerLeft.SM_TrackCornerLeft")))

(event Custom|CorrectSplineAfterDirection
  (params (Direction :type E_Direction%20Enum :default "NewEnumerator1"))
  (bind _returnvalue (Math|Conversions|ToInteger(Byte) Direction))
  (bind _station (Variables|References|GetStation))
  (bind _spawnpoints (Variables|PlacementNodes|GetSpawnPoints))
  (bind _splinetangentmag (Variables|Spline|GetSplineTangentMag))
  (bind _output (Utilities|Array|Get(acopy) _spawnpoints _returnvalue))
  (bind _spline (Variables|/Game/UltraRail/Blueprints/Track/BP_StartStation.BP_StartStation_C|GetSpline _station))
  (bind _returnvalue_2 (Math|Vector|GetForwardVector _output))
  ;[1 1 1] Updates the spline point to correspond with the direction
  (if (!= (Variables|Spline|GetSplineIndex) 0)
    (Spline|SetLocationatSplinePoint _spline (Variables|Spline|GetSplineIndex) (Transformation|GetWorldLocation _output) "World" true)
    (Spline|SetTangentsatSplinePoint _spline (Variables|Spline|GetSplineIndex) (* _returnvalue_2 _splinetangentmag) (* _returnvalue_2 _splinetangentmag) "World" true)))

(event EventBeginPlay
  ;[1 1 1] Set all placement spawn points in array and set startstaion
  (Variables|PlacementNodes|SetSpawnPoints (Utilities|Array|MakeArray (Variables|Default|GetStraight) (Variables|Default|GetRight) (Variables|Default|GetLeft)))
  (bind _returnvalue (Actor|GetActorOfClass "/Game/UltraRail/Blueprints/Track/BP_StartStation.BP_StartStation_C"))
  (Variables|References|SetStation _returnvalue))

(fn ConstructionScript)

(fn StringtoDirection
  (params (Name :type String%20%28by%20ref%29))
  (bind _rights (Utilities|String|Split Name "."))
  (bind _stringtoenummap (Variables|PlacementNodes|GetStringToEnumMap))
  (bind (_value _returnvalue) (Utilities|Map|Find _stringtoenummap _rights))
  ;[1 1 1] Set string to direction enum
  (if _returnvalue
    (return _value)
    (else
      (Development|PrintString "String not in map" true true "(R=1.000000,G=0.000000,B=0.000000,A=1.000000)" 2e+01))))