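; End station that links player-placed track to its built-in track pieces and handles the train's arrival.
; Forward and right placement triggers lock the placed piece and chain the child-actor tracks' splines onto it, with the right side first rotating and redirecting the first piece.
; Connecting changes the locomotive's max speed to hurry it in.
; The arrival trigger brakes it, restores its saved top speed, marks the new last track and broadcasts OnTrainArrived.
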(event OnComponentBeginOverlap(RailsPlacementTriggerForward)
  (params (OverlappedComponent :type Primitive%20Component%20Object%20Reference) (OtherActor :type Actor%20Object%20Reference) (OtherComp :type Primitive%20Component%20Object%20Reference) (OtherBodyIndex :type Integer) (bFromSweep :type Boolean) (SweepResult :type Hit%20Result%20Structure%20%28by%20ref%29))
  ;[1 1 1] Triggers the tracks to connect when a trackpiece is placed at the correct position
  (if (Class|GameplayStatics|ObjectIsA OtherActor (Variables|Check|GetTrackCheckType))
    (CallFunction|ChangePickup (.AsBP%20Track (Utilities|Casting|CastToBP_Track OtherActor)))
    (Utilities|FlowControl|DelayUntilNextTick)
    (CallFunction|CoupleSplines)
    (CallFunction|DestroyTriggers)
    (CallFunction|SpeedupTrain)))

(event OnComponentBeginOverlap(ArrivalTrigger)
  (params (OverlappedComponent :type Primitive%20Component%20Object%20Reference) (OtherActor :type Actor%20Object%20Reference) (OtherComp :type Primitive%20Component%20Object%20Reference) (OtherBodyIndex :type Integer) (bFromSweep :type Boolean) (SweepResult :type Hit%20Result%20Structure%20%28by%20ref%29))
  (bind _asbp_locomotive (Utilities|Casting|CastToBP_Locomotive OtherActor))
  ;[1 1 1] Force the train to brake harder and notify listeners that a train has arrived
  (if (Class|GameplayStatics|ObjectIsA OtherActor (Variables|Check|GetTrainCheckType))
    (Default|SetBrakingForce _asbp_locomotive (Default|GetTopSpeed _asbp_locomotive))
    (CallFunction|RestoreTrainSpeed)
    (Variables|/Game/UltraRail/Blueprints/Track/BP_Track.BP_Track_C|SetIsLast (.AsBP%20Track (Utilities|Casting|CastToBP_Track (Variables|/Script/Engine.ChildActorComponent|GetChildActor (Variables|Default|GetTrack4)))) true)
    (Default|CallOnTrainArrived self _asbp_locomotive)
    (Components|DestroyComponent (Variables|Default|GetArrivalTrigger))))

(event OnComponentBeginOverlap(RailsPlacementTriggerRight)
  (params (OverlappedComponent :type Primitive%20Component%20Object%20Reference) (OtherActor :type Actor%20Object%20Reference) (OtherComp :type Primitive%20Component%20Object%20Reference) (OtherBodyIndex :type Integer) (bFromSweep :type Boolean) (SweepResult :type Hit%20Result%20Structure%20%28by%20ref%29))
  (bind _track1 (Variables|Default|GetTrack1))
  (bind _childactor (Variables|/Script/Engine.ChildActorComponent|GetChildActor _track1))
  (bind _asbp_track (Utilities|Casting|CastToBP_Track _childactor))
  ;[1 1 1] Updates the first track piece and corrects the spline
  (if (Class|GameplayStatics|ObjectIsA OtherActor (Variables|Check|GetTrackCheckType))
    (CallFunction|ChangePickup (.AsBP%20Track (Utilities|Casting|CastToBP_Track OtherActor)))
    (Transformation|SetRelativeLocationAndRotation _track1 (Math|Vector|RotateVectorAroundAxis (Variables|/Script/Engine.SceneComponent|GetRelativeLocation _track1) -9e+01 "0.000000,0.000000,1.000000") "0.000000,-90.000000,0.000000" false true)
    (Default|SetMeshDirection _asbp_track "NewEnumerator2")
    (Utilities|FlowControl|DelayUntilNextTick)
    (CallFunction|CoupleSplines)
    (Default|CorrectSplineAfterDirection _asbp_track "NewEnumerator2")
    (CallFunction|DestroyTriggers)
    (CallFunction|SpeedupTrain)))

(event Custom|ChangePickup
  (params (TrackPiece :type BP%20Track%20Object%20Reference))
  ;[1 1 1] Change the pickup rules of the last placed piece
  (bind _output_get (Variables|Default|SetPlacedPiece TrackPiece))
  (Variables|/Game/UltraRail/Blueprints/Track/BP_Track.BP_Track_C|SetCanBePickedUp _output_get false)
  (Variables|/Game/UltraRail/Blueprints/Track/BP_Track.BP_Track_C|SetIsLast (Variables|Default|GetPlacedPiece) false))

(event Custom|CoupleSplines
  (bind _track1 (Variables|Default|GetTrack1))
  (bind _track2 (Variables|Default|GetTrack2))
  (bind _childactor (Variables|/Script/Engine.ChildActorComponent|GetChildActor _track1))
  (bind _childactor_2 (Variables|/Script/Engine.ChildActorComponent|GetChildActor _track2))
  (bind _asbp_track (Utilities|Casting|CastToBP_Track _childactor))
  (bind _asbp_track_2 (Utilities|Casting|CastToBP_Track _childactor_2))
  ;[1 1 1] Couples the spline with that from the original starting station
  (Default|OnPlace _asbp_track (Variables|Default|GetPlacedPiece))
  (Default|OnPlace _asbp_track_2 _asbp_track)
  (Default|OnPlace (.AsBP%20Track (Utilities|Casting|CastToBP_Track (Variables|/Script/Engine.ChildActorComponent|GetChildActor (Variables|Default|GetTrack3)))) _asbp_track_2)
  (Default|OnPlace (.AsBP%20Track (Utilities|Casting|CastToBP_Track (Variables|/Script/Engine.ChildActorComponent|GetChildActor (Variables|Default|GetTrack4)))) _asbp_track_2))

(event Custom|DestroyTriggers
  ;[1 1 1] Destroys the track-placement triggers
  (Components|DestroyComponent (Variables|Default|GetRailsPlacementTriggerRight)))

(event Custom|SpeedupTrain
  (bind _train (Variables|Default|GetTrain))
  ;[1 1 1] Speed-up the train when the rail has been connected al the way up to the station
  (Variables|Speed|SetLastTrainSpeed (Default|GetTopSpeed _train))
  (Default|SetMaxSpeed _train 1.2))

(event Custom|RestoreTrainSpeed
  ;[1 1 1] Restores the train previous top speed
  (Default|SetMaxSpeed (Variables|Default|GetTrain) (Variables|Speed|GetLastTrainSpeed)))

(event EventBeginPlay
  ;[1 1 1] Get the train at the start
  (bind _returnvalue (Actor|GetActorOfClass "/Game/UltraRail/Blueprints/Train/BP_Locomotive.BP_Locomotive_C"))
  (Variables|Default|SetTrain _returnvalue))

(fn ConstructionScript)