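; BP_PlacementNode is a placement node owned by a BP_Track that previews a hologram mesh for the player.
; Each tick it evaluates the hologram only while its track is the last one, and destroys itself if the owner is invalid.
; The hologram shows when an overlapping top-down character holds a specific item, faces within 45 degrees, and CheckCollision finds no blocking actors outside a class filter.
; Turning away or ending overlap hides it.
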(event OnComponentEndOverlap(PlayerChackBox)
  (params (OverlappedComponent :type Primitive%20Component%20Object%20Reference) (OtherActor :type Actor%20Object%20Reference) (OtherComp :type Primitive%20Component%20Object%20Reference) (OtherBodyIndex :type Integer))
  ;[1 1 1] Check for collision for when to deactivate the hologram
  (CallFunction|DeactivateHologram))

(event Custom|ActivateHologram
  (bind _playerchackbox (Variables|Default|GetPlayerChackBox))
  (bind _holostaticmesh (Variables|Default|GetHoloStaticMesh))
  (bind _overlappingactors (Collision|GetOverlappingActors _playerchackbox "/Game/UltraRail/Blueprints/Core/BP_TopDownCharacter.BP_TopDownCharacter_C" :!class /Script/Engine.PrimitiveComponent))
  ;[1 1 1] Activates the hologram when there is no collision and the player is looking in the same direction
  (for _array_element _overlappingactors
    (bind _asbp_top_down_character (Utilities|Casting|CastToBP_TopDownCharacter _array_element))
    (if (Utilities|Enum|Equal(Enum) (Variables|/Game/UltraRail/Blueprints/Core/BP_TopDownCharacter.BP_TopDownCharacter_C|GetItem _asbp_top_down_character) "NewEnumerator1")
      (bind _sucsses (CallFunction|CheckCollision))
      (if (not _sucsses)
        (if (Utilities|Array|IsNotEmpty _overlappingactors)
          (for _array_element_2 _overlappingactors
            (bind _asbp_top_down_character_2 (Utilities|Casting|CastToBP_TopDownCharacter _array_element_2))
            (if (and (Utilities|Operators|EqualEqual (Transformation|GetWorldRotation (Variables|/Script/Engine.Character|GetCapsuleComponent _asbp_top_down_character_2)) (Transformation|GetWorldRotation (Variables|Default|GetDefaultSceneRoot)) 45.0) (not (Variables|Default|GetCollision)))
              (Rendering|SetVisibility _holostaticmesh true false)
              (Development|SetHiddeninGame _holostaticmesh false false)))
          (else
            (CallFunction|DeactivateHologram)))))))

(event Custom|DeactivateHologram
  (bind _holostaticmesh (Variables|Default|GetHoloStaticMesh))
  ;[1 1 1] Deactivates the hologram
  (Rendering|SetVisibility _holostaticmesh false false)
  (Development|SetHiddeninGame _holostaticmesh true false))

(event EventBeginPlay
  ;[1 1 1] Sets the hologram static mesh, material and activates the hologram
  (Components|StaticMesh|SetStaticMesh (Variables|Default|GetHoloStaticMesh) (Variables|Default|GetStaticMeshHologram))
  (Rendering|Material|SetMaterial (Variables|Default|GetHoloStaticMesh) 0 (Variables|Default|GetMaterialHologram))
  (CallFunction|ActivateHologram))

(event EventTick
  (params (DeltaSeconds :type Float%20%28single-precision%29))
  (bind _returnvalue (Components|GetOwner))
  ;[1 1 1] Activates the hologram when the player is near and looking in the same direction as the hologram is
  (Utilities|IsValid _returnvalue
    (:Is%20Valid
      (bind _asbp_track (Utilities|Casting|CastToBP_Track _returnvalue))
      (if (Variables|/Game/UltraRail/Blueprints/Track/BP_Track.BP_Track_C|GetIsLast _asbp_track)
        (CallFunction|ActivateHologram)
        (for _array_element (Collision|GetOverlappingActors (Variables|Default|GetPlayerChackBox) "/Game/UltraRail/Blueprints/Core/BP_TopDownCharacter.BP_TopDownCharacter_C" :!class /Script/Engine.PrimitiveComponent)
          (bind _asbp_top_down_character (Utilities|Casting|CastToBP_TopDownCharacter _array_element))
          (if (not (Utilities|Operators|EqualEqual (Transformation|GetWorldRotation (Variables|/Script/Engine.Character|GetCapsuleComponent _asbp_top_down_character)) (Transformation|GetWorldRotation (Variables|Default|GetDefaultSceneRoot)) 45.0))
            (CallFunction|DeactivateHologram)))
        (else
          (CallFunction|DeactivateHologram))))
    (:Is%20Not%20Valid
      (Actor|DestroyActor))))

(fn ConstructionScript)

(fn CheckCollision
  (bind _collionbox (Variables|Default|GetCollionBox))
  (bind _overlappingactors (Collision|GetOverlappingActors _collionbox 0 :!class /Script/Engine.PrimitiveComponent))
  ;[1 1 1] Checks if there is collision
  (if (Utilities|Array|IsNotEmpty _overlappingactors)
    (for _array_element _overlappingactors
      (bind _wasfound (CallFunction|ClassFilter (Variables|Default|GetFilterlist) (Utilities|GetClass _array_element)))
      (if _wasfound
        (Variables|Default|SetCollision false)
        (else
          (bind _output_get (Variables|Default|SetCollision true))
          (return _output_get))))
    (return false)))