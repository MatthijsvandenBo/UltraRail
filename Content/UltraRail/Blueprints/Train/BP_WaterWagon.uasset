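; BP_WaterWagon is a train wagon that tracks a water supply and can be refilled with buckets.
; It starts at full capacity, and Tick runs the parent logic, then swaps the tank mesh once when water falls to a fifth of maximum.
; Overlapping its box with a filled BP_Bucket restores capacity, sets the bucket's empty mesh and the original tank mesh, and calls ExtinguishFire.
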(event OnComponentBeginOverlap(Box)
  (params (OverlappedComponent :type Primitive%20Component%20Object%20Reference) (OtherActor :type Actor%20Object%20Reference) (OtherComp :type Primitive%20Component%20Object%20Reference) (OtherBodyIndex :type Integer) (bFromSweep :type Boolean) (SweepResult :type Hit%20Result%20Structure%20%28by%20ref%29))
  ;[1 1 1] If a full bucket is presented then we reset the water capacity and extinguish the fire
  (bind _asbp_bucket (Utilities|Casting|CastToBP_Bucket OtherActor))
  (if (Variables|/Game/UltraRail/Blueprints/Tools/BP_Bucket.BP_Bucket_C|GetHasWater _asbp_bucket)
    (Variables|Default|SetWaterCapacity (Variables|Default|GetMaxWaterCapacity))
    (Components|StaticMesh|SetStaticMesh (Variables|/Game/UltraRail/Blueprints/BP_PickUpMain.BP_PickUpMain_C|GetStaticMesh _asbp_bucket) "/Game/UltraRail/Art/Assets/Tools/BucketEmpty.BucketEmpty")
    (Components|StaticMesh|SetStaticMesh (Variables|Default|GetWagonTop) "/Game/UltraRail/Art/Assets/Trains/NS2100/NS2100WaterTank1.NS2100WaterTank1")
    (CallFunction|ExtinguishFire _asbp_bucket)))

(event EventBeginPlay
  ;[1 1 1] Sets the initial water capacity
  (|CallParentFunction)
  (Variables|Default|SetWaterCapacity (Variables|Default|GetMaxWaterCapacity)))

(event EventTick
  (params (DeltaSeconds :type Float%20%28single-precision%29))
  ;[1 1 1] Moves the water wagon
  (|CallParentFunction DeltaSeconds)
  (if (<= (Variables|Default|GetWaterCapacity) (* (Variables|Default|GetMaxWaterCapacity) 0.2))
    (Utilities|FlowControl|DoOnce false :!label _label
      (:Completed
        (Components|StaticMesh|SetStaticMesh (Variables|Default|GetWagonTop) "/Game/UltraRail/Art/Assets/Trains/NS2100/NS2100WaterTank2.NS2100WaterTank2")))
    (else
      (goto _label Reset))))

(fn ConstructionScript
  (|CallParentFunction))