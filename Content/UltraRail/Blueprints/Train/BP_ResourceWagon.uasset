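; Resource wagon of the train that carries a wood pile and an iron pile, both stackable objects spawned as child actors.
; On train assembly it binds to each pile's added-to-stack event, which unhides that pile and fires the wagon's own AddedToStack dispatcher.
; It exposes both stack amounts and removes one from each pile together.
; Ticking defers to the parent, and a bucket overlapping its box extinguishes fire.
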(event OnComponentBeginOverlap(Box)
  (params (OverlappedComponent :type Primitive%20Component%20Object%20Reference) (OtherActor :type Actor%20Object%20Reference) (OtherComp :type Primitive%20Component%20Object%20Reference) (OtherBodyIndex :type Integer) (bFromSweep :type Boolean) (SweepResult :type Hit%20Result%20Structure%20%28by%20ref%29))
  ;[1 1 1] Call Extinguish fire when bucket is presented
  (bind _asbp_bucket (Utilities|Casting|CastToBP_Bucket OtherActor))
  (CallFunction|ExtinguishFire _asbp_bucket))

(event Custom|AddedWoodToStack
  ;[1 1 1] adds to the stacks
  (Rendering|SetActorHiddenInGame (Variables|Refrences|GetWoodPile) false)
  (Default|CallAddedtoStack))

(event Custom|RemoveFromStack
  ;[1 1 1] removes from both stacks and the stackable objects
  (Default|RemovefromStack (Variables|Refrences|GetWoodPile) 1))

(event Custom|AddedIronToStack
  ;[1 1 1] adds to the stacks
  (Rendering|SetActorHiddenInGame (Variables|Refrences|GetIronPile) false)
  (Default|CallAddedtoStack))

(event EventTrainAssembled
  (params (Locomotive :type BP%20Locomotive%20Object%20Reference))
  ;[1 1 1] adds to the stacks
  (bind _asbp_stackable_object (Utilities|Casting|CastToBP_StackableObject (Variables|/Script/Engine.ChildActorComponent|GetChildActor (Variables|Default|GetWoodPileObject))))
  (bind _output_get (Variables|Refrences|SetWoodPile _asbp_stackable_object))
  (EventDispatchers|BindEventtoAddedtoStack _output_get (EventDispatchers|CreateEvent :!event Custom|AddedWoodToStack))
  (bind _asbp_stackable_object_2 (Utilities|Casting|CastToBP_StackableObject (Variables|/Script/Engine.ChildActorComponent|GetChildActor (Variables|Default|GetIronPileObject))))
  (bind _output_get_2 (Variables|Refrences|SetIronPile _asbp_stackable_object_2))
  (EventDispatchers|BindEventtoAddedtoStack _output_get_2 (EventDispatchers|CreateEvent :!event Custom|AddedIronToStack)))

(event EventTick
  (params (DeltaSeconds :type Float%20%28single-precision%29))
  ;[1 1 1] moves the wagon
  (|CallParentFunction DeltaSeconds))

(fn ConstructionScript
  (|CallParentFunction))

(fn GetWoodStackAmount
  ;[1 1 1] Returns the amount on the wood pile
  (return (Variables|/Game/UltraRail/Blueprints/Resources/BP_StackableObject.BP_StackableObject_C|GetAmountOnStack (Variables|Refrences|GetWoodPile))))

(fn GetIronStackAmount
  ;[1 1 1] Returns the amount on the iron pile
  (return (Variables|/Game/UltraRail/Blueprints/Resources/BP_StackableObject.BP_StackableObject_C|GetAmountOnStack (Variables|Refrences|GetIronPile))))