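; BP_PlacementNode shows a hologram at a spot where a track piece could be placed in the train game.
; While its owning BP_Track is the last one, Tick re-evaluates the hologram; otherwise it hides it.
; The hologram appears when an overlapping BP_TopDownCharacter carries track, roughly matches the node's rotation, and the collision box holds only actors of filtered classes.
; It hides when the character turns away or an overlap with the player check box ends.
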(event OnComponentEndOverlap(PlayerChackBox)
  (params (OverlappedComponent :type Primitive%20Component%20Object%20Reference) (OtherActor :type Actor%20Object%20Reference) (OtherComp :type Primitive%20Component%20Object%20Reference) (OtherBodyIndex :type Integer))
  (CallFunction|DeactivateHologram))

(event Custom|ActivateHologram
  (bind _playerchackbox (Variables|Default|GetPlayerChackBox))
  (bind _holostaticmesh (Variables|Default|GetHoloStaticMesh))
  (bind _holostaticmesh_2 (Variables|Default|GetHoloStaticMesh))
  (bind _overlappingactors (Collision|GetOverlappingActors _playerchackbox "/Game/UltraRail/Blueprints/BP_TopDownCharacter.BP_TopDownCharacter_C" :!class /Script/Engine.PrimitiveComponent))
  (for _array_element _overlappingactors
    (bind _asbp_top_down_character (Utilities|Casting|CastToBP_TopDownCharacter _array_element))
    (if (Variables|/Game/UltraRail/Blueprints/BP_TopDownCharacter.BP_TopDownCharacter_C|GetHasTrack _asbp_top_down_character)
      (bind _sucsses (CallFunction|CheckCollision))
      (if (not _sucsses)
        (if (Utilities|Array|IsNotEmpty _overlappingactors)
          (for _array_element_2 _overlappingactors
            (bind _asbp_top_down_character_2 (Utilities|Casting|CastToBP_TopDownCharacter _array_element_2))
            (if (and (Utilities|Operators|EqualEqual (Transformation|GetWorldRotation (Variables|/Script/Engine.Character|GetCapsuleComponent _asbp_top_down_character_2)) (Transformation|GetWorldRotation (Variables|Default|GetDefaultSceneRoot)) 45.0) (not (Variables|Default|GetCollision)))
              (Rendering|SetVisibility _holostaticmesh_2 true false)
              (Development|SetHiddeninGame _holostaticmesh_2 false false)))
          (else
            (Rendering|SetVisibility _holostaticmesh false false)
            (Development|SetHiddeninGame _holostaticmesh true false)))))))

(event Custom|DeactivateHologram
  (bind _holostaticmesh (Variables|Default|GetHoloStaticMesh))
  (Rendering|SetVisibility _holostaticmesh false false)
  (Development|SetHiddeninGame _holostaticmesh true false))

(event EventBeginPlay
  (Components|StaticMesh|SetStaticMesh (Variables|Default|GetHoloStaticMesh) (Variables|Default|GetStaticMeshHologram))
  (Rendering|Material|SetMaterial (Variables|Default|GetHoloStaticMesh) 0 (Variables|Default|GetMaterialHologram))
  (CallFunction|ActivateHologram))

(event EventTick
  (params (DeltaSeconds :type Float%20%28single-precision%29))
  (bind _asbp_track (Utilities|Casting|CastToBP_Track (Components|GetOwner)))
  (if (Variables|/Game/UltraRail/Blueprints/Train/BP_Track.BP_Track_C|GetIsLast _asbp_track)
    (CallFunction|ActivateHologram)
    (for _array_element (Collision|GetOverlappingActors (Variables|Default|GetPlayerChackBox) "/Game/UltraRail/Blueprints/BP_TopDownCharacter.BP_TopDownCharacter_C" :!class /Script/Engine.PrimitiveComponent)
      (bind _asbp_top_down_character (Utilities|Casting|CastToBP_TopDownCharacter _array_element))
      (if (not (Utilities|Operators|EqualEqual (Transformation|GetWorldRotation (Variables|/Script/Engine.Character|GetCapsuleComponent _asbp_top_down_character)) (Transformation|GetWorldRotation (Variables|Default|GetDefaultSceneRoot)) 45.0))
        (CallFunction|DeactivateHologram)))
    (else
      (CallFunction|DeactivateHologram))))

(fn ConstructionScript)

(fn CheckCollision
  (bind _collionbox (Variables|Default|GetCollionBox))
  (bind _overlappingactors (Collision|GetOverlappingActors _collionbox 0 :!class /Script/Engine.PrimitiveComponent))
  (if (Utilities|Array|IsNotEmpty _overlappingactors)
    (for _array_element _overlappingactors
      (bind _wasfound (CallFunction|ClassFilter (Utilities|GetClass _array_element)))
      (if _wasfound
        (Variables|Default|SetCollision false)
        (else
          (bind _output_get (Variables|Default|SetCollision true))
          (return _output_get))))))

(fn ClassFilter
  (params (TestClass :type Object%20Class%20Reference))
  (for _array_element (Variables|Default|GetFilterlist)
    (if (Utilities|ClassIsChildOf TestClass _array_element)
      (return true)))
  (return false))