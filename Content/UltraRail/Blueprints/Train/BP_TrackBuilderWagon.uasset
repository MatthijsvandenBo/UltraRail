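; BP_TrackBuilderWagon is a train wagon that forges track pieces from wood and iron held in storage wagons.
; BeginPlay gathers all storage wagons, starts a looping forge timer and makes its child-actor track stack indestructible.
; Forging looks for a wagon holding both materials, adds a track to the stack if below the maximum, then removes materials.
; Tick syncs the track count with the stack.
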(event Custom|StartForging
  (bind _trackstack (Variables|Default|GetTrackStack))
  ;[1 1 1] Craft the rail and then uses the materials needed, spawns it on top of the wagon
  (bind (_array_element _array_index) (Utilities|Array|ForEachLoopwithBreak (Variables|Default|GetStorageWagons) :!label _label)
    (:LoopBody
      (if (and (> (Variables|/Game/UltraRail/Blueprints/Train/BP_StorageWagon.BP_StorageWagon_C|GetCurrentWoodStack _array_element) 0) (> (Variables|/Game/UltraRail/Blueprints/Train/BP_StorageWagon.BP_StorageWagon_C|GetCurrentIronStack _array_element) 0))
        (Variables|Default|SetArrayIndex _array_index)
        (goto _label Break)))
    (:Completed
      (if (Math|Boolean|ANDBoolean (>= (Variables|/Game/UltraRail/Blueprints/Train/BP_StorageWagon.BP_StorageWagon_C|GetCurrentWoodStack (Utilities|Array|Get(acopy) (Variables|Default|GetStorageWagons) (Variables|Default|GetArrayIndex))) 1) (>= (Variables|/Game/UltraRail/Blueprints/Train/BP_StorageWagon.BP_StorageWagon_C|GetCurrentIronStack (Utilities|Array|Get(acopy) (Variables|Default|GetStorageWagons) (Variables|Default|GetArrayIndex))) 1) (< (Variables|Default|GetTracks) (Variables|Default|GetMaxTrackStack)))
        (Variables|/Game/UltraRail/Blueprints/Resources/BP_StackableObject.BP_StackableObject_C|SetAmountToAdd _trackstack 1)
        (Default|AddtoStack _trackstack)
        (Math|Integer|IncrementInt (Variables|Default|GetTracks)
          (:%20%20
            (Default|RemovefromStack (Utilities|Array|Get(acopy) (Variables|Default|GetStorageWagons) (Variables|Default|GetArrayIndex)))))))))

(event EventBeginPlay
  ;[1 1 1] Gets refrences and starts crafting timer
  (|CallParentFunction)
  (bind _outactors (Actor|GetAllActorsOfClass "/Game/UltraRail/Blueprints/Train/BP_StorageWagon.BP_StorageWagon_C"))
  (Variables|Default|SetStorageWagons _outactors)
  (Utilities|Time|SetTimerbyEvent (EventDispatchers|CreateEvent :!event Custom|StartForging) (Variables|Default|GetForgeDuration) true true)
  (bind _asbp_stackable_object (Utilities|Casting|CastToBP_StackableObject (Variables|/Script/Engine.ChildActorComponent|GetChildActor (Variables|Default|GetTrackStackableObject))))
  (Variables|Default|SetTrackStack _asbp_stackable_object)
  (Variables|/Game/UltraRail/Blueprints/Resources/BP_StackableObject.BP_StackableObject_C|SetCanBeDestroyed _asbp_stackable_object false))

(event EventTick
  (params (DeltaSeconds :type Float%20%28single-precision%29))
  (bind _trackstack (Variables|Default|GetTrackStack))
  ;[1 1 1] Moves the wagon and removes tracks when the player picks them up
  (|CallParentFunction DeltaSeconds)
  (Utilities|IsValid _trackstack
    (:Is%20Valid
      (Variables|Default|SetTracks (Variables|/Game/UltraRail/Blueprints/Resources/BP_StackableObject.BP_StackableObject_C|GetAmountOnStack _trackstack)))))

(fn ConstructionScript
  (|CallParentFunction))