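; BP_TrackTraverser is an actor that moves along the start station's track spline and can catch fire, apparently as a base for train parts.
; Track position is a spline input key that sets actor location and the yaw of a rotating target.
; Progress only advances forward while not burning; a water-filled bucket clears the fire flag and empties.
; It spawns a hidden fire emitter and provides a near-end check and a default zero speed.
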(event Custom|ExtinguishFire
  (params (Bucket :type BP%20Bucket%20Object%20Reference))
  ;[1 1 1] Puts out the fire when presented with a full bucket
  (if (Variables|/Game/UltraRail/Blueprints/Tools/BP_Bucket.BP_Bucket_C|GetHasWater Bucket)
    (Variables|Default|SetIsOnFire false)
    (Variables|/Game/UltraRail/Blueprints/Tools/BP_Bucket.BP_Bucket_C|SetHasWater Bucket false)))

(event EventBeginPlay
  ;[1 1 1] Gets the track-spline from the starting station
  (bind _returnvalue (Actor|GetActorOfClass "/Game/UltraRail/Blueprints/Track/BP_StartStation.BP_StartStation_C"))
  (Variables|Track|SetTrackSpline (Variables|/Game/UltraRail/Blueprints/Track/BP_StartStation.BP_StartStation_C|GetSpline _returnvalue))
  (bind _returnvalue_2 (Effects|SpawnEmitterAttached "/Game/StarterContent/Particles/P_Fire.P_Fire" (Variables|Default|GetDefaultSceneRoot) "None"))
  (bind _output_get (Variables|Default|SetFireEffect _returnvalue_2))
  (Rendering|SetVisibility _output_get false false))

(fn ConstructionScript)

(fn GetCurrentTrackPosition
  ;[1 1 1] Returns the current track-position
  (return (Variables|Track|GetTrackPosition)))

(fn SetTrackPosition
  (params (NewValue :type Float%20%28double-precision%29))
  (bind (_location _rotation) (CallFunction|GetPositionalLocation))
  ;[1 1 1] Sets the track position
  (Variables|Track|SetTrackPosition NewValue)
  (Transformation|SetActorLocation _location false false)
  (Transformation|SetWorldRotation (Variables|Default|GetRotatingTarget) (Math|Rotator|MakeRotator 0.0 0.0 (.yaw _rotation)) false false)
  (return))

(fn GetPositionalLocation
  (bind _trackspline (Variables|Track|GetTrackSpline))
  (bind _trackposition (Variables|Track|GetTrackPosition))
  (bind _returnvalue (Class|SplineComponent|GetTransformatSplineInputKey _trackspline _trackposition "World" false))
  ;[1 1 1] Gets the world location from the given track position on the spline
  (return (.location _returnvalue) (.rotation _returnvalue)))

(fn AddtoProgress
  (params (DeltaProgress :type Float%20%28double-precision%29))
  ;[1 1 1] Adds to the current progress
  (if (not (Variables|Default|GetIsOnFire))
    (if (> DeltaProgress 0.0)
      (CallFunction|SetTrackPosition (+ (Variables|Track|GetTrackPosition) DeltaProgress))
      (return))))

(fn GetTrackSpline
  ;[1 1 1] Returns the reference to the track spline
  (return (Variables|Track|GetTrackSpline)))

(fn GetCurrentSpeed
  ;[1 1 1] Default implementation for getting the current speed
  (return 0.0))

(fn IsNearEnd
  (params (DetectionError :type Float%20%28double-precision%29))
  ;[1 1 1] Checks if the traverser is nearing the end of the track
  (return (< (- (Spline|GetNumberOfSplinePoints (Variables|Track|GetTrackSpline)) (Variables|Track|GetTrackPosition)) DetectionError)))