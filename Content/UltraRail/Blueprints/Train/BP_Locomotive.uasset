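; Locomotive actor that accelerates along the track up to a max speed, using inherited progress movement with its mesh as the rotating target.
; Each tick it draws cooling water from the level's water wagons; without water it catches fire and brakes, which blocks acceleration.
; An overlapping bucket triggers fire extinguishing.
; Test code destroys the train near track end while it has water.
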(event OnComponentBeginOverlap(Box)
  (params (OverlappedComponent :type Primitive%20Component%20Object%20Reference) (OtherActor :type Actor%20Object%20Reference) (OtherComp :type Primitive%20Component%20Object%20Reference) (OtherBodyIndex :type Integer) (bFromSweep :type Boolean) (SweepResult :type Hit%20Result%20Structure%20%28by%20ref%29))
  (bind _asbp_bucket (Utilities|Casting|CastToBP_Bucket OtherActor))
  (CallFunction|ExtinguishFire _asbp_bucket))

(event Custom|SetBrakingForce
  (params (NewBakingForce :type Float%20%28double-precision%29))
  ;[1 1 1] Sets the braking force
  (Variables|Movement|SetBrakingForce (Math|Float|Max(Float) NewBakingForce 0.0)))

(event Custom|AddAcceleration
  (params (IncreaseAmount :type Float%20%28double-precision%29))
  ;[1 1 1] Adds acceleration to train
  ;;[0 0 0] Ignore acceleration when the braking force is greater than 0
  (if (not (> (Variables|Movement|GetBrakingForce) 0.0))
    (Variables|Movement|SetCurrentSpeed (Math|Float|Min(Float) (+ (Variables|Movement|GetCurrentSpeed) IncreaseAmount) (Variables|Movement|GetMaxSpeed)))))

(event Custom|ApplyBrakingForce
  (params (DeltaTime :type Float%20%28double-precision%29))
  ;[1 1 1] Adds bracking force to train
  (Variables|Movement|SetCurrentSpeed (Math|Float|Max(Float) (- (Variables|Movement|GetCurrentSpeed) (* (Variables|Movement|GetBrakingForce) DeltaTime)) 0.0)))

(event Custom|SetMaxSpeed
  (params (NewMaxSpeed :type Float%20%28double-precision%29))
  ;[1 1 1] Sets the max speed
  (Variables|Movement|SetMaxSpeed (Math|Float|Max(Float) NewMaxSpeed 0.0)))

(event EventBeginPlay
  ;[1 1 1] Set the train mesh as the rotating target
  (|CallParentFunction)
  (Variables|Default|SetRotatingTarget (Variables|Default|GetTrainMesh))
  (bind _outactors (Actor|GetAllActorsOfClass "/Game/UltraRail/Blueprints/Train/BP_WaterWagon.BP_WaterWagon_C"))
  (Variables|Default|SetWaterWagons _outactors))

(event EventTick
  (params (DeltaSeconds :type Float%20%28single-precision%29))
  ;[1 1 1] Moves the train along the track
  (|CallParentFunction DeltaSeconds)
  (CallFunction|AddAcceleration (* (Variables|Movement|GetAcceleration) DeltaSeconds))
  (CallFunction|AddtoProgress (* (Variables|Movement|GetCurrentSpeed) DeltaSeconds))
  (CallFunction|ApplyBrakingForce DeltaSeconds)
  ;[1 1 1] Controls the fire and cooling of the train
  (for (_array_element _array_index) (Variables|Default|GetWaterWagons)
    (if (> (Variables|/Game/UltraRail/Blueprints/Train/BP_WaterWagon.BP_WaterWagon_C|GetWaterCapacity _array_element) 0)
      (Variables|Default|SetArray%20Index _array_index)
      (else
        (Variables|Default|SetArray%20Index -1))))
  (if (!= (Variables|Default|GetArray%20Index) -1)
    (Math|Integer|DecrementInt (Variables|/Game/UltraRail/Blueprints/Train/BP_WaterWagon.BP_WaterWagon_C|GetWaterCapacity (Utilities|Array|Get(acopy) (Variables|Default|GetWaterWagons) (Variables|Default|GetArray%20Index)))
      (:%20%20
        (CallFunction|SetBrakingForce 0.0)
        ;[0 0 1] Kills the train at end of track (Test-code)
        (if (CallFunction|IsNearEnd 1.5)
          (Actor|DestroyActor))))
    (else
      (Variables|Default|SetIsOnFire true)
      (CallFunction|SetBrakingForce 1.0))))

(fn ConstructionScript)

(fn GetCurrentSpeed
  ;[1 1 1] Returns the current speed of the locomotive
  (return (Variables|Movement|GetCurrentSpeed)))

(fn GetTopSpeed
  ;[1 1 1] Returns the top speed
  (return (Variables|Movement|GetMaxSpeed)))