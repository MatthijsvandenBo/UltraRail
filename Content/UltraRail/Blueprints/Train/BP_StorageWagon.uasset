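; BP_StorageWagon is a train wagon that stores wood and iron in two stackable piles, with movement left to its parent class.
; On BeginPlay it makes both child-actor BP_StackableObject piles indestructible and binds to their added-to-stack events.
; Each addition raises that resource's counter only if the whole amount fits under the shared MaxStack limit.
; RemoveFromStack takes one from both piles and both counters together.
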(event Custom|AddedToIronStack
  ;[1 1 1] adds to the stacks
  (if (and (<= (Variables|/Game/UltraRail/Blueprints/Resources/BP_StackableObject.BP_StackableObject_C|GetAmountToAdd (stale EventBeginPlay _asbp_stackable_object_2)) (- (Variables|Default|GetMaxStack) (Variables|Default|GetCurrentIronStack))) (< (Variables|Default|GetCurrentIronStack) (Variables|Default|GetMaxStack)))
    (Variables|Default|SetCurrentIronStack (+ (Variables|/Game/UltraRail/Blueprints/Resources/BP_StackableObject.BP_StackableObject_C|GetAmountToAdd (stale EventBeginPlay _asbp_stackable_object_2)) (Variables|Default|GetCurrentIronStack)))))

(event Custom|AddedToWoodStack
  ;[1 1 1] adds to the stacks
  (if (and (<= (Variables|/Game/UltraRail/Blueprints/Resources/BP_StackableObject.BP_StackableObject_C|GetAmountToAdd (stale EventBeginPlay _asbp_stackable_object)) (- (Variables|Default|GetMaxStack) (Variables|Default|GetCurrentWoodStack))) (< (Variables|Default|GetCurrentWoodStack) (Variables|Default|GetMaxStack)))
    (Variables|Default|SetCurrentWoodStack (+ (Variables|/Game/UltraRail/Blueprints/Resources/BP_StackableObject.BP_StackableObject_C|GetAmountToAdd (stale EventBeginPlay _asbp_stackable_object)) (Variables|Default|GetCurrentWoodStack)))))

(event Custom|RemoveFromStack
  ;[1 1 1] removes from both stacks and the stackable objects
  (Default|RemovefromStack (.AsBP%20Stackable%20Object (Utilities|Casting|CastToBP_StackableObject (Variables|/Script/Engine.ChildActorComponent|GetChildActor (Variables|Default|GetWoodPile)))) 1)
  (Math|Integer|DecrementInt (Variables|Default|GetCurrentIronStack)
    (:%20%20
      (Math|Integer|DecrementInt (Variables|Default|GetCurrentWoodStack)))))

(event EventBeginPlay
  ;[1 1 1] adds to the stacks
  (|CallParentFunction)
  (bind _asbp_stackable_object (Utilities|Casting|CastToBP_StackableObject (Variables|/Script/Engine.ChildActorComponent|GetChildActor (Variables|Default|GetWoodPile))))
  (Variables|/Game/UltraRail/Blueprints/Resources/BP_StackableObject.BP_StackableObject_C|SetCanBeDestroyed _asbp_stackable_object false)
  (EventDispatchers|BindEventtoAddedtoStack _asbp_stackable_object (delegate Custom|AddedToWoodStack))
  (bind _asbp_stackable_object_2 (Utilities|Casting|CastToBP_StackableObject (Variables|/Script/Engine.ChildActorComponent|GetChildActor (Variables|Default|GetIronPile))))
  (Variables|/Game/UltraRail/Blueprints/Resources/BP_StackableObject.BP_StackableObject_C|SetCanBeDestroyed _asbp_stackable_object_2 false)
  (EventDispatchers|BindEventtoAddedtoStack _asbp_stackable_object_2 (delegate Custom|AddedToIronStack)))

(event EventTick
  (params (DeltaSeconds :type Float%20%28single-precision%29))
  ;[1 1 1] moves the wagon
  (|CallParentFunction DeltaSeconds))

(fn ConstructionScript
  (|CallParentFunction))