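; BP_Track is a placeable rail piece that extends the train route along the spline owned by BP_StartStaion.
; On placement it spawns straight, right and left placement nodes with hologram meshes, updates the previous piece and appends a spline point.
; The previous piece takes its straight or corner mesh from the node with a visible hologram, then moves its spline point and sets tangents to match that direction.
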(event Custom|OnPlace
  (params (OldTrack :type BP%20Track%20Object%20Reference))
  (bind _station (Variables|Default|GetStation))
  (bind _spline (Variables|/Game/UltraRail/Blueprints/Train/BP_StartStaion.BP_StartStaion_C|GetSpline _station))
  ;[1 1 1] Spawns all placement nodes and put them in a array
  (bind _output_get (Variables|Default|SetPreviousTrackpiece OldTrack))
  (for _array_element (Variables|Default|GetSpawnPionts)
    (bind _returnvalue (Game|SpawnActorfromClass "/Game/UltraRail/Blueprints/Train/BP_PlacementNode.BP_PlacementNode_C" (Math|Transform|MakeTransform (Transformation|GetWorldLocation _array_element) (Transformation|GetWorldRotation _array_element) "1.000000,1.000000,1.000000") "Undefined" "MultiplyWithRoot" self "/Game/UltraRail/Models/SM_Track.SM_Track" (CallFunction|SetDirection (Utilities|GetDisplayName _array_element)) 0))
    (Utilities|Array|Add (Variables|Default|GetPlacementNodes) _returnvalue))
  ;[1 1 1] Update's track and adds spline point
  (Utilities|IsValid _output_get
    (:Is%20Valid
      (CallFunction|UpdatePreviousTrackpiece _output_get)
      (Spline|AddSplinePoint _spline (Transformation|GetWorldLocation (Variables|Default|GetStraight)) "World" true)
      (Variables|Default|SetSplineIndex (- (Spline|GetNumberOfSplinePoints _spline) 1)))))

(event Custom|UpdatePreviousTrackpiece
  (bind _splinetangentmag (Variables|Default|GetSplineTangentMag))
  (bind _station (Variables|Default|GetStation))
  (bind _spline (Variables|/Game/UltraRail/Blueprints/Train/BP_StartStaion.BP_StartStaion_C|GetSpline _station))
  ;[1 1 1] Sets the mesh of the track and change's the spline point
  (for _array_element (Variables|Default|GetPlacementNodes)
    (if (Rendering|IsVisible (Variables|/Game/UltraRail/Blueprints/Train/BP_PlacementNode.BP_PlacementNode_C|GetHoloStaticMesh _array_element))
      (Components|StaticMesh|SetStaticMesh (Variables|Default|GetStaticMesh) (Utilities|Select :Index (Variables|/Game/UltraRail/Blueprints/Train/BP_PlacementNode.BP_PlacementNode_C|GetDirection _array_element) :NewEnumerator1 "/Game/UltraRail/Models/SM_Track.SM_Track" :NewEnumerator2 "/Game/UltraRail/Models/SM_TrackCornerRight.SM_TrackCornerRight" :NewEnumerator0 "/Game/UltraRail/Models/SM_TrackCornerLeft.SM_TrackCornerLeft"))
      (Spline|SetLocationatSplinePoint _spline (Variables|Default|GetSplineIndex) (Transformation|GetWorldLocation (Utilities|Array|Get(acopy) (Variables|Default|GetSpawnPionts) (Math|Conversions|ToInteger(Byte) (Variables|/Game/UltraRail/Blueprints/Train/BP_PlacementNode.BP_PlacementNode_C|GetDirection _array_element)))) "World" true)
      (Spline|SetTangentsatSplinePoint _spline (Variables|Default|GetSplineIndex) (* (Math|Vector|GetForwardVector (Transformation|GetWorldRotation (Utilities|Array|Get(acopy) (Variables|Default|GetSpawnPionts) (Math|Conversions|ToInteger(Byte) (Variables|/Game/UltraRail/Blueprints/Train/BP_PlacementNode.BP_PlacementNode_C|GetDirection _array_element))))) _splinetangentmag) (* (Math|Vector|GetForwardVector (Transformation|GetWorldRotation (Utilities|Array|Get(acopy) (Variables|Default|GetSpawnPionts) (Math|Conversions|ToInteger(Byte) (Variables|/Game/UltraRail/Blueprints/Train/BP_PlacementNode.BP_PlacementNode_C|GetDirection _array_element))))) _splinetangentmag) "World" true))))

(event EventBeginPlay
  ;[1 1 1] Set all placement spawn points in array and set startstaion
  (Variables|Default|SetSpawnPionts (Utilities|Array|MakeArray (Variables|Default|GetStraight) (Variables|Default|GetRight) (Variables|Default|GetLeft)))
  (bind _returnvalue (Actor|GetActorOfClass "/Game/UltraRail/Blueprints/Train/BP_StartStaion.BP_StartStaion_C"))
  (Variables|Default|SetStation _returnvalue))

(fn ConstructionScript)

(fn SetDirection
  (params (Name :type String%20%28by%20ref%29))
  (bind _rights (Utilities|String|Split Name "."))
  (bind _stringtoenummap (Variables|Default|GetStringToEnumMap))
  (bind (_value _returnvalue) (Utilities|Map|Find _stringtoenummap _rights))
  (if _returnvalue
    (return _value)
    (else
      (Development|PrintString "Hello"))))