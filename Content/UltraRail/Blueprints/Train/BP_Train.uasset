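; BP_Train is the train actor that runs along the spline of the BP_StartStation found at BeginPlay.
; Each tick it integrates speed into a spline input key, setting location and mesh yaw from it.
; Acceleration is capped at max speed and ignored while braking force is positive; braking slows it no lower than zero.
; When its front point nears the spline's end, it destroys itself and calls OnGameEnd.
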(event Custom|AddAcceleration
  (params (IncreaseAmount :type Float%20%28double-precision%29))
  ;[1 1 1] Adds acceleration to train
  ;;[1 1 1] Ignore acceleration when the braking force is greater than 0
  (if (not (> (Variables|Default|GetBrakingForce) 0.0))
    (Variables|Default|SetCurrentSpeed (Math|Float|Min(Float) (+ (Variables|Default|GetCurrentSpeed) IncreaseAmount) (Variables|Default|GetMaxSpeed)))))

(event Custom|ApplyBrakingForce
  (params (DeltaTime :type Float%20%28double-precision%29))
  ;[1 1 1] Adds bracking force to train
  (Variables|Default|SetCurrentSpeed (Math|Float|Max(Float) (- (Variables|Default|GetCurrentSpeed) (* (Variables|Default|GetBrakingForce) DeltaTime)) 0.0)))

(event EventBeginPlay
  ;[1 1 1] Get spline
  (bind _returnvalue (Actor|GetActorOfClass "/Game/UltraRail/Blueprints/Track/BP_StartStation.BP_StartStation_C"))
  (Variables|Default|SetSpline (Variables|/Game/UltraRail/Blueprints/Track/BP_StartStation.BP_StartStation_C|GetSpline _returnvalue)))

(event EventTick
  (params (DeltaSeconds :type Float%20%28single-precision%29))
  (bind _spline (Variables|Default|GetSpline))
  ;[1 1 1] moves the train
  (CallFunction|AddAcceleration (* (Variables|Default|GetAcceleration) DeltaSeconds))
  (bind _output_get (Variables|Default|SetPosition (+ (Variables|Default|GetPosition) (* (Variables|Default|GetCurrentSpeed) DeltaSeconds))))
  (Transformation|SetActorLocation (.location (Class|SplineComponent|GetTransformatSplineInputKey (Variables|Default|GetSpline) _output_get "World" false)) false false)
  (Transformation|SetWorldRotation (Variables|Default|GetTrainMesh) (Math|Rotator|MakeRotator 0.0 0.0 (.yaw (.rotation (Class|SplineComponent|GetTransformatSplineInputKey (Variables|Default|GetSpline) _output_get "World" false)))) false false)
  (CallFunction|ApplyBrakingForce DeltaSeconds)
  (if (Utilities|Operators|EqualEqual (Transformation|GetWorldLocation (Variables|Default|GetFrontPoint)) (Class|SplineComponent|GetLocationatSplineInputKey _spline (Spline|GetSplineLength _spline) "World") 1e+01)
    (Actor|DestroyActor)
    (Default|CallOnGameEnd)))

(fn ConstructionScript)