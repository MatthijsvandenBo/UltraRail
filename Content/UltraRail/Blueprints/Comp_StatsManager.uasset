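; Actor component that tracks the farthest distance its owner has travelled along the world Y axis from where it began play.
; BeginPlay stores the starting Y position, divided by 100, as the baseline.
; Each tick it recomputes the offset from that baseline and, only on a new maximum, saves it and broadcasts OnDistanceUpdated.
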(event EventBeginPlay
  ;[1 1 1] Initialize the start distance
  (Variables|Default|SetStartDistance (CallFunction|CalculateDistance)))

(event EventTick
  (params (DeltaSeconds :type Float%20%28single-precision%29))
  ;[1 1 1] Update the distance if it is higher than the previous distance
  (if (> (CallFunction|CalculateDistance) (Variables|Default|GetDistance))
    (bind _output_get (Variables|Default|SetDistance (CallFunction|CalculateDistance)))
    (Default|CallOnDistanceUpdated _output_get)))

(fn CalculateDistance
  ;[1 1 1] Calculate the distance from the start distance
  (return (- (/ (.y (Transformation|GetActorLocation (Components|GetOwner))) 100) (Variables|Default|GetStartDistance))))