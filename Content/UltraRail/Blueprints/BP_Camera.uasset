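; Main camera that trails the train along the world Y axis.
; On BeginPlay it becomes player 0's view target and polls until a BP_Train exists.
; Each tick it eases its root toward the train's CamPoint only when that point is at greater Y, so it never moves back; X and Z stay unchanged.
; Smoothstep is actually a lerp using clamped delta time as alpha.
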(event EventBeginPlay
  ;[1 1 1] Set main camera and gets train
  (Game|Player|SetViewTargetwithBlend (Game|GetPlayerController 0) self 0.0 "VTBlend_Linear" 0.0 false)
  (bind _object (Utilities|WaitUntilClassValid "/Game/UltraRail/Blueprints/Train/BP_Train.BP_Train_C" 0.1 100)
    (:Success
      (Variables|Default|SetTrain (.AsBP%20Train (Utilities|Casting|CastToBP_Train _object))))))

(event EventTick
  (params (DeltaSeconds :type Float%20%28single-precision%29))
  (bind _defaultsceneroot (Variables|Default|GetDefaultSceneRoot))
  (bind _returnvalue (Transformation|GetWorldLocation _defaultsceneroot))
  ;[1 1 1] Set the cam location to the train
  (bind _train (Variables|Default|GetTrain)
    (:then
      (bind _should (CallFunction|ShouldFollow _train))
      (if _should
        (Transformation|SetWorldLocation (Variables|Default|GetDefaultSceneRoot) (Math|Vector|MakeVector (.x _returnvalue) (CallFunction|Smoothstep (.y _returnvalue) (.y (Transformation|GetWorldLocation (Variables|/Game/UltraRail/Blueprints/Train/BP_Train.BP_Train_C|GetCamPoint _train))) DeltaSeconds) (.z _returnvalue)) false false)))
    (:else)))

(fn ConstructionScript)

(fn Smoothstep
  (params (Value :type Float%20%28double-precision%29) (Target :type Float%20%28double-precision%29) (DeltaTime :type Float%20%28double-precision%29))
  ;[1 1 1] Smoothsteps between values
  (return (Math|Float|Lerp Value Target (Math|Float|Clamp(Float) DeltaTime))))

(fn ShouldFollow
  (params (Train :type BP%20Train%20Object%20Reference))
  ;[1 1 1] Returns wether the camera should or should not follow the train at the given moment
  (return (> (.y (Transformation|GetWorldLocation (Variables|/Game/UltraRail/Blueprints/Train/BP_Train.BP_Train_C|GetCamPoint Train))) (.y (Transformation|GetWorldLocation (Variables|Default|GetDefaultSceneRoot))))))