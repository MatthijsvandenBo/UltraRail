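; BP_Bucket is a placeable bucket tool that fills with water and shows a full or empty mesh to match.
; Overlapping a BP_WaterBlock sets HasWater and swaps to the filled mesh, which BeginPlay also applies if the bucket already holds water.
; Tick watches HasWater through two DoOnce gates that reset each other, so the mesh swaps only when the state changes.
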(event OnComponentBeginOverlap(StaticMesh)
  (params (OverlappedComponent :type Primitive%20Component%20Object%20Reference) (OtherActor :type Actor%20Object%20Reference) (OtherComp :type Primitive%20Component%20Object%20Reference) (OtherBodyIndex :type Integer) (bFromSweep :type Boolean) (SweepResult :type Hit%20Result%20Structure%20%28by%20ref%29))
  ;[1 1 1] Gets the water into he bucket
  (if (Class|GameplayStatics|ObjectIsA OtherActor "/Game/UltraRail/Blueprints/Blocks/BP_WaterBlock.BP_WaterBlock_C")
    (Components|StaticMesh|SetStaticMesh (Variables|Default|GetStaticMesh) "/Game/UltraRail/Art/Assets/Tools/Bucket.Bucket")
    (Variables|Default|SetHasWater true)))

(event EventBeginPlay
  ;[1 1 1] sets the mesh when placed down by player
  (|CallParentFunction)
  (if (Variables|Default|GetHasWater)
    (Components|StaticMesh|SetStaticMesh (Variables|Default|GetStaticMesh) "/Game/UltraRail/Art/Assets/Tools/Bucket.Bucket")))

(event EventTick
  (params (DeltaSeconds :type Float%20%28single-precision%29))
  ;[1 1 1] sets the correct mesh
  (if (Variables|Default|GetHasWater)
    (Utilities|FlowControl|DoOnce false :!label _label
      (:Completed
        (Components|StaticMesh|SetStaticMesh (Variables|Default|GetStaticMesh) "/Game/UltraRail/Art/Assets/Tools/Bucket.Bucket")
        (goto _label_2 Reset)))
    (else
      (Utilities|FlowControl|DoOnce false :!label _label_2
        (:Completed
          (Components|StaticMesh|SetStaticMesh (Variables|Default|GetStaticMesh) "/Game/UltraRail/Art/Assets/Tools/BucketEmpty.BucketEmpty")
          (goto _label Reset))))))

(fn ConstructionScript
  (|CallParentFunction))