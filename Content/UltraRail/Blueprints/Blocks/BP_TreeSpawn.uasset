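; BP_TreeSpawn is a block Blueprint that places a tree on a randomly chosen block mesh.
; On BeginPlay it sets BlockMesh to a random static mesh from AllowedBlocks, then spawns a BP_Tree at the world location of TreeSpawnPoint.
; The tree always spawns regardless of collision, and the construction script only calls its parent.
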(event Custom|SpawnTree
  ;[1 1 1] Spawns in the tree
  (Game|SpawnActorfromClass "/Game/UltraRail/Blueprints/Resources/BP_Tree.BP_Tree_C" (Math|Transform|MakeTransform (Transformation|GetWorldLocation (Variables|Default|GetTreeSpawnPoint)) "0, 0, 0" "1.000000,1.000000,1.000000") "AlwaysSpawn" "MultiplyWithRoot" 0 0))

(event Custom|SpawnBlock
  ;[1 1 1] Spawns in a random block from the given allowed blocks
  (Components|StaticMesh|SetStaticMesh (Variables|Default|GetBlockMesh) (.OutItem (Utilities|Array|Random (Variables|Default|GetAllowedBlocks)))))

(event EventBeginPlay
  (CallFunction|SpawnBlock)
  (CallFunction|SpawnTree))

(fn ConstructionScript
  (|CallParentFunction))